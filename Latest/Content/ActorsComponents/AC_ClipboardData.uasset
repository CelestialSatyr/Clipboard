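; AC_ClipboardData is an actor component that manages the personal clipboard widget and marks itself for saving.
; On BeginPlay it fetches the Clipboard subsystem actor; creating the widget registers it there, refreshes it and shows it.
; Toggle and force-remove events add or remove the widget and switch between clipboard and game input modes, with cleanup on EndPlay.
; Save hooks need no transform and declare no dependencies.
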(event EventEndPlay
  (params (EndPlayReason :type EEndPlayReason%20Enum :default "Destroyed"))
  (Utilities|IsValid (Variables|Default|GetWidgetReference)
    (:Is%20Valid
      (Widget|RemovefromParent (Variables|Default|GetWidgetReference))
      (Variables|Default|SetWidgetReference 0))))

(event EventBeginPlay
  (Variables|Default|SetClipboardSubsystem (Class|SubsystemActorManager|GetSubsystemActor (Subsystems|GetSubsystemActorManager) "/CDevClipboard/Subsystem_Clipboard.Subsystem_Clipboard_C")))

(event EventForceRemoveWidget
  (Widget|RemovefromParent (Variables|Default|GetWidgetReference))
  (CallFunction|ReturnModetoGame))

(event EventCreateWidget
  (bind _clipboardsubsystem (Variables|Default|GetClipboardSubsystem))
  (bind _returnvalue (UserInterface|CreateWidget "/CDevClipboard/Widgets/Widget_PersonalClipboard.Widget_PersonalClipboard_C"))
  (bind _output_get (Variables|Default|SetWidgetReference _returnvalue))
  (Default|SetWidgetReference _clipboardsubsystem _output_get)
  (Default|RefreshWidget _clipboardsubsystem)
  (UserInterface|Viewport|AddtoViewport _output_get 0)
  (CallFunction|SetModetoClipboard (Variables|Default|GetWidgetReference)))

(event EventToggleWidget
  (bind _widgetreference (Variables|Default|GetWidgetReference))
  (if (Widget|IsVisible _widgetreference)
    (Widget|RemovefromParent _widgetreference)
    (CallFunction|ReturnModetoGame)
    (else
      (UserInterface|Viewport|AddtoViewport _widgetreference 0)
      (CallFunction|SetModetoClipboard (Variables|Default|GetWidgetReference)))))

(fn GatherDependencies
  (return 0))

(fn GetNextDataEntryID
  (return 0))

(fn HasAvailableWidget
  (return (Utilities|IsValid (Variables|Default|GetWidgetReference))))

(fn NeedTransform
  (return false))

(fn ShouldSave
  (return true))